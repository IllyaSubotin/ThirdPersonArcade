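; AI_Actor is an enemy pawn that endlessly chases the player and deals damage on reaching them.
; BeginPlay runs a move-to loop that applies damage on each success, then restarts after a short delay; a failed move ends the loop.
; Taking damage lowers Health, awarding BP_Character XP and destroying the actor at zero.
; Surviving hits briefly set a negative walk speed and swap the cube's material without restoring it.
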(event `self.ReceiveBeginPlay`
  (bind _returnvalue (`GameplayStatics.GetPlayerCharacter` 0))
  (`|AIMoveTo` self (0.0 0.0 0.0) _returnvalue 30.0 :!label _label
    (:`OnSuccess`
      (`GameplayStatics.ApplyDamage` _returnvalue 5.0)
      (bind _asbp_character (cast `/Game/Blueprint/Core/BP_Character` (`GameplayStatics.GetPlayerCharacter` 0)))
      (set `/Game/Blueprint/Core/BP_Character.XP` (`/Game/Blueprint/Core/BP_Character.XP` _asbp_character) _asbp_character)
      (`KismetSystemLibrary.Delay` 0.1)
      (goto _label))))

(event `self.ReceiveAnyDamage`
  (params (Damage :type "Float (single-precision)") (DamageType :type "DamageType Object Reference") (InstigatedBy :type "Controller Object Reference") (DamageCauser :type "Actor Object Reference"))
  (bind _charactermovement (`self.CharacterMovement`))
  (bind _output_get (set `self.Health` (- (`self.Health`) Damage)))
  (if (<= _output_get 0.0)
    (bind _asbp_character (cast `/Game/Blueprint/Core/BP_Character` (`GameplayStatics.GetPlayerCharacter` 0)))
    (set `/Game/Blueprint/Core/BP_Character.XP` (+ (`/Game/Blueprint/Core/BP_Character.XP` _asbp_character) 5.0) _asbp_character)
    (`self.K2_DestroyActor`)
    (else
      (set `CharacterMovementComponent.MaxWalkSpeed` -100.0 _charactermovement)
      (`PrimitiveComponent.SetMaterial` (`self.Cube`) 0 "/Game/Materials/Paladin_MAT.Paladin_MAT")
      (`KismetSystemLibrary.Delay` 0.2)
      (set `CharacterMovementComponent.MaxWalkSpeed` 100.0 _charactermovement))))

(fn `UserConstructionScript`)