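; BP_Character is the player character, with camera-relative movement, yaw look, sprinting, health and XP levelling.
; On BeginPlay it spawns a BP_Sword on the mesh's Sword_joint socket.
; Attacking while stationary sets IsAttack and briefly locks movement, while attacking on the move plays a montage.
; Tick raises stats when XP fills, and damage briefly swaps the material or opens MainMenu at zero health.
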(event `self.ReceiveBeginPlay`
  ;[1 1 1] SwordJoin
  (bind _returnvalue (`|SpawnActorFromClass` "/Game/Blueprint/SWord/BP_Sword.BP_Sword_C" (`SceneComponent.GetSocketTransform` (`self.Mesh`) "Sword_joint" "RTS_World") "Undefined" "OverrideRootScale" null null))
  (`self.K2_AttachToComponent` _returnvalue (`self.Mesh`) "Sword_joint" "SnapToTarget" "SnapToTarget" "SnapToTarget" true))

(event `InputAxis|InputAxis_Forward`
  (params (AxisValue :type "Float (single-precision)"))
  (bind (_returnvalue_roll _returnvalue_pitch _returnvalue_yaw) (`KismetMathLibrary.BreakRotator` (`self.GetControlRotation`)))
  ;[1 1 1] Move
  (`self.AddMovementInput` (`KismetMathLibrary.GetForwardVector` (`KismetMathLibrary.MakeRotator` 0.0 0.0 _returnvalue_yaw)) AxisValue))

(event `InputAxis|InputAxis_X`
  (params (AxisValue :type "Float (single-precision)"))
  ;[1 1 1] Camera
  (`self.AddControllerYawInput` AxisValue))

(event `InputAxis|InputAxis_RightLeft`
  (params (AxisValue :type "Float (single-precision)"))
  (bind (_returnvalue_roll _returnvalue_pitch _returnvalue_yaw) (`KismetMathLibrary.BreakRotator` (`self.GetControlRotation`)))
  ;[1 1 1] Move
  (`self.AddMovementInput` (`KismetMathLibrary.GetRightVector` (`KismetMathLibrary.MakeRotator` _returnvalue_roll 0.0 _returnvalue_yaw)) AxisValue))

(event `InputAction|InputAction_attack`
  (params (Key :type "Key Structure"))
  (bind _charactermovement (`self.CharacterMovement`))
  ;[1 1 1] Attack1
  (:`Pressed`
    (if (== (`KismetMathLibrary.VSize` (`self.GetVelocity`)) 0.0)
      (set `self.IsAttack` true)
      (set `CharacterMovementComponent.MaxWalkSpeed` 0.0 _charactermovement)
      (`KismetSystemLibrary.Delay` 1.2)
      (set `self.IsAttack` false)
      (set `CharacterMovementComponent.MaxWalkSpeed` 600.0 _charactermovement)
      (else
        (`self.PlayAnimMontage` "/Game/Animation/Montage_Attack1.Montage_Attack1")))))

(event `InputAction|InputAction_run`
  (params (Key :type "Key Structure"))
  ;[1 1 1] Move
  (:`Pressed`
    (set `CharacterMovementComponent.MaxWalkSpeed` 2000.0 (`self.CharacterMovement`))))

(event `InputAction|InputAction_Walk`
  (params (Key :type "Key Structure"))
  ;[1 1 1] Move
  (:`Released`
    (set `CharacterMovementComponent.MaxWalkSpeed` 600.0 (`self.CharacterMovement`))))

(event `self.ReceiveTick`
  (params (DeltaSeconds :type "Float (single-precision)"))
  (if (>= (`self.XP`) (`self.maxXP`))
    (set `self.maxXP` (+ (`self.maxXP`) 5.0))
    (set `self.maxHealth` (+ (`self.maxHealth`) 20.0))
    (set `self.damage` (+ (`self.damage`) 2.0))
    (set `self.health` (+ (`self.health`) 20.0))
    (set `self.XP` 0.0)))

(event `self.ReceiveAnyDamage`
  (params (Damage :type "Float (single-precision)") (DamageType :type "DamageType Object Reference") (InstigatedBy :type "Controller Object Reference") (DamageCauser :type "Actor Object Reference"))
  ;[1 1 1] Take Damage
  (set `self.health` (- (`self.health`) Damage))
  (if (<= (`self.health`) 0.0)
    (`GameplayStatics.OpenLevel` "MainMenu")
    (else
      (`PrimitiveComponent.SetMaterial` (`self.Mesh`) 0 "/Game/Materials/Paladin_MAT2.Paladin_MAT2")
      (`KismetSystemLibrary.Delay` 0.3)
      (`PrimitiveComponent.SetMaterial` (`self.Mesh`) 0 "/Game/Materials/Paladin_MAT.Paladin_MAT"))))

(fn `StopSprint`
  (set `CharacterMovementComponent.MaxWalkSpeed` 600.0 (`self.CharacterMovement`)))

(fn `UserConstructionScript`)